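; Puzzle cube activator that the player rotates in 90-degree steps when nearby.
; Box overlap sets CanRotate for any actor and shows the BP_KeyF prompt widget for Characters; leaving reverses both.
; The RotateCube input, enabled on BeginPlay, turns the cube and cycles ActualValue through four states.
; Each turn asks RotatorsManager, when valid, to check the rotators' answer.
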(event `InputAction|RotateCube` :consume false
  (params (Key :type "Key Structure"))
  (bind _rotatorsmanager (`self.rotatorsManager`))
  ;[1 1 1] Tourne le cube à 90° sur l'axe X et vérifie la réponse du joueur en envoyant les informations au manager
  ;;[1 1 1] Si la variable "can rotate" est à true, tourne le cube
  (:`Pressed`
    (if (`self.canRotate`)
      (`self.K2_AddActorLocalRotation` (struct :`Roll` 90.0))
      ;;[1 1 1] Incrémente la valeur de l'objet actuel. Si cette dernière dépasse 4, la remet à 0.
      (bind _output_get (set `self.actualValue` (+ (`self.actualValue`) 1)))
      (if (== _output_get 4)
        (set `self.actualValue` 0))
      ;;[1 1 1] Vérifie si le manager est toujours valide. Si oui, envoie la réponse du joueur au manager pour vérification
      (if (`KismetSystemLibrary.IsValid` _rotatorsmanager)
        (`/Game/BP/Managers/RotatorCubesManager.CheckRotators` _rotatorsmanager)))))

(event `self.Box.OnComponentBeginOverlap`
  (params (OverlappedComponent :type "PrimitiveComponent Object Reference") (OtherActor :type "Actor Object Reference") (OtherComp :type "PrimitiveComponent Object Reference") (OtherBodyIndex :type Integer) (bFromSweep :type Boolean) (SweepResult :type "HitResult Structure (by ref)"))
  ;[1 1 1] Affiche une image si le joueur est proche (indication touche à appuyer) et met la variable "can rotate" à true
  (set `self.canRotate` true)
  (cast `Character` OtherActor)
  (bind _returnvalue (`|CreateWidget` "/Game/BP/UI/BP_KeyF.BP_KeyF_C"))
  (`UserWidget.AddToViewport` _returnvalue 0))

(event `self.ReceiveBeginPlay`
  ;[1 1 1] Active l'utilisation des "inputs" et reset de la valeur "can rotate)
  (`self.EnableInput` (`GameplayStatics.GetPlayerController` 0))
  (set `self.canRotate` false))

(event `self.Box.OnComponentEndOverlap`
  (params (OverlappedComponent :type "PrimitiveComponent Object Reference") (OtherActor :type "Actor Object Reference") (OtherComp :type "PrimitiveComponent Object Reference") (OtherBodyIndex :type Integer))
  ;[1 1 1] Enlève l'image affichée si le joueur s'éloigne et met la variable "can rotate" à false
  (set `self.canRotate` false)
  (cast `Character` OtherActor)
  (`Widget.RemoveFromParent` (stale `self.Box.OnComponentBeginOverlap` _returnvalue)))

(fn `UserConstructionScript`)